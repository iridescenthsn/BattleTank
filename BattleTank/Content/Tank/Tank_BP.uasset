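; Tank_BP is the player-controllable tank pawn that wires input to its aiming and movement components.
; On BeginPlay it initializes TankAiming with the turret and barrel, and TankMovement with the left and right tracks.
; Aim axes rotate the AzimuthGambil and SpringArm camera rig, move and turn axes send intents to TankMovement, and the Fire action calls Fire.
; Debug prints mark construction and BeginPlay.
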(event EventBeginPlay
  (Development|PrintString "donkey: BP begin play called")
  (Class|TankAimingComponent|Intialize (Variables|Default|GetTankAiming) (Variables|Default|GetTankTurret) (Variables|Default|GetTankBarrel))
  (Class|TankMovementComponent|Intialize (Variables|Default|GetTankMovement) (Variables|Default|GetLeft%20Track) (Variables|Default|GetRight%20Track)))

(event Input|ActionEvents|InputActionFire
  (params (Key :type Key%20Structure :default "None"))
  ;[1 1 1] aim Setup
  (:Pressed
    (Class|Tank|Fire)))

(event Input|AxisEvents|InputAxisAimAzimuth
  (params (AxisValue :type Float%20%28single-precision%29))
  ;[1 1 1] aim Setup
  (Transformation|AddLocalRotation (Variables|Default|GetAzimuth%20gambil) (Math|Rotator|MakeRotator 0.0 0.0 AxisValue) false false))

(event Input|AxisEvents|InputAxisAimAltitude
  (params (AxisValue :type Float%20%28single-precision%29))
  ;[1 1 1] aim Setup
  (Transformation|AddLocalRotation (Variables|Default|GetSpringArm) (Math|Rotator|MakeRotator 0.0 AxisValue 0.0) false false))

(event Input|AxisEvents|InputAxisMoveForward
  (params (AxisValue :type Float%20%28single-precision%29))
  (Class|TankMovementComponent|IntendMoveForward (Variables|Default|GetTankMovement) AxisValue))

(event Input|AxisEvents|InputAxisTurnRight
  (params (AxisValue :type Float%20%28single-precision%29))
  (Class|TankMovementComponent|IntendTurnRight (Variables|Default|GetTankMovement) AxisValue))

(fn ConstructionScript
  (Development|PrintString "BP constructor called"))